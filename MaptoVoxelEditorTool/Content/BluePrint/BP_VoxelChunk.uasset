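; Voxel chunk actor that stores occupancy and renders it as voxel instances or per-group billboards.
; AddVoxelChunk marks each voxel in a mask, sorts it into 4x4x4 groups and optionally adds a HISM cube.
; BuildGroupsBillboard packs each group's 64 voxels into four 16-bit masks, passed as custom data on camera-facing HISM billboards.
; AddHoudiniBillboard adds billboards from precomputed masks, also passing group position as custom data.
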(fn `AddHoudiniBillboard`
  (params (GroupX :type Integer) (GroupY :type Integer) (GroupZ :type Integer) (Mask0 :type Integer) (Mask1 :type Integer) (Mask2 :type Integer) (Mask3 :type Integer) (CamLoc :type "Vector Structure") (CamRo :type "Rotator Structure"))
  (bind _hism_groupbillboard (`self.HISM_GroupBillboard`))
  (bind _returnvalue (`KismetMathLibrary.MakeVector` (* (+ (* (`KismetMathLibrary.Conv_IntToDouble` GroupX) 4.0) 1.5) 100.0) (* (+ (* (`KismetMathLibrary.Conv_IntToDouble` GroupY) 4.0) 1.5) 100.0) (* (+ (* (`KismetMathLibrary.Conv_IntToDouble` GroupZ) 4.0) 1.5) 100.0)))
  (`KismetSystemLibrary.PrintString` "Called!")
  (bind _returnvalue_2 (`InstancedStaticMeshComponent.AddInstance` (`self.HISM_GroupBillboard`) (`KismetMathLibrary.MakeTransform` _returnvalue (`KismetMathLibrary.ComposeRotators` (`KismetMathLibrary.FindLookAtRotation` _returnvalue CamLoc) (struct :`Pitch` 90.0 :`Roll` 30.0)) (`KismetMathLibrary.MakeVector` 4.0 4.0 1.0)) false))
  (`InstancedStaticMeshComponent.SetCustomDataValue` _hism_groupbillboard _returnvalue_2 0 (`KismetMathLibrary.Conv_IntToDouble` Mask0) false)
  (`InstancedStaticMeshComponent.SetCustomDataValue` _hism_groupbillboard _returnvalue_2 1 (`KismetMathLibrary.Conv_IntToDouble` Mask1) false)
  (`InstancedStaticMeshComponent.SetCustomDataValue` _hism_groupbillboard _returnvalue_2 2 (`KismetMathLibrary.Conv_IntToDouble` Mask2) false)
  (`InstancedStaticMeshComponent.SetCustomDataValue` _hism_groupbillboard _returnvalue_2 3 (`KismetMathLibrary.Conv_IntToDouble` Mask3) true)
  (`InstancedStaticMeshComponent.SetCustomDataValue` _hism_groupbillboard _returnvalue_2 4 (.x _returnvalue) true)
  (`InstancedStaticMeshComponent.SetCustomDataValue` _hism_groupbillboard _returnvalue_2 5 (.y _returnvalue) true)
  (`InstancedStaticMeshComponent.SetCustomDataValue` _hism_groupbillboard _returnvalue_2 6 (.z _returnvalue) true))

(fn `AddVoxelChunk`
  (params (Transform :type "Transform Structure") (VoxelData :type "/Game/BluePrint/Data/ST_VoxelData Structure") (ShowVoxels :type Boolean))
  (locals (Mask0 :type Integer) (Mask1 :type Integer) (Mask2 :type Boolean) (Mask3 :type Boolean))
  (bind (_occupied _gridx _gridy _gridz) (break `/Game/BluePrint/Data/ST_VoxelData` VoxelData))
  (bind _chunksize (`self.ChunkSize`))
  (bind _tempvoxelindices (`self.TempVoxelIndices`))
  (bind _groupdataarray (`self.GroupDataArray`))
  (bind _returnvalue (`KismetMathLibrary.FTrunc` _chunksize))
  (bind _returnvalue_2 (/ (`self.ChunkSize`) 4))
  (bind _returnvalue_3 (mod _gridx _returnvalue))
  (bind _returnvalue_4 (mod _gridy _returnvalue))
  (bind _returnvalue_5 (mod _gridz _returnvalue))
  (bind _returnvalue_6 (/ _returnvalue_3 4))
  (bind _returnvalue_7 (/ _returnvalue_5 4))
  (bind _returnvalue_8 (/ _returnvalue_4 4))
  (bind _returnvalue_9 (+ _returnvalue_3 (* _returnvalue_4 _chunksize) (* _returnvalue_5 _chunksize _chunksize)))
  (bind _returnvalue_10 (+ _returnvalue_6 (* _returnvalue_8 _returnvalue_2) (* _returnvalue_7 _returnvalue_2 _returnvalue_2)))
  (`KismetArrayLibrary.Array_Set` (`self.VoxelMask`) _returnvalue_9 true true)
  (if (not (`KismetArrayLibrary.Array_Contains` (`self.GroupKey`) _returnvalue_10))
    (`KismetArrayLibrary.Array_Add` (`self.GroupKey`) _returnvalue_10)
    (`KismetArrayLibrary.Array_Add` _groupdataarray (make `/Game/BluePrint/Data/ST_GroupData` _returnvalue_10 _returnvalue_6 _returnvalue_8 _returnvalue_7)))
  (for (_array_element _array_index) _groupdataarray
    (bind (_groupindex _groupx _groupy _groupz _voxelindices) (break `/Game/BluePrint/Data/ST_GroupData` _array_element))
    (if (== _groupindex _returnvalue_10)
      (bind _output_get (set `self.TempVoxelIndices` _voxelindices))
      (`KismetArrayLibrary.Array_AddUnique` _output_get _returnvalue_9)
      (`KismetArrayLibrary.Array_Set` (`self.GroupDataArray`) _array_index (make `/Game/BluePrint/Data/ST_GroupData` _groupindex _groupx _groupy _groupz _tempvoxelindices))
      (`KismetSystemLibrary.PrintString` (`KismetStringLibrary.Conv_IntToString` (`KismetArrayLibrary.Array_Length` _tempvoxelindices)))
      (`KismetSystemLibrary.PrintString` (`KismetStringLibrary.Conv_IntToString` _groupindex))))
  (if ShowVoxels
    (`InstancedStaticMeshComponent.AddInstance` (`self.HISM_Voxel`) Transform true)))

(fn `BuildGroupsBillboard`
  (params (VoxelDataArray :type "Array of /Game/BluePrint/Data/ST_VoxelData Structure") (ShowBillboards :type Boolean))
  (locals (Mask0 :type "Float (double-precision)") (Mask1 :type "Float (double-precision)") (Mask2 :type "Float (double-precision)") (Mask3 :type "Float (double-precision)"))
  (bind _voxelsize (`self.VoxelSize`))
  (bind _returnvalue (`KismetMathLibrary.FTrunc` (`self.ChunkSize`)))
  (bind _returnvalue_2 (/ (* (`self.VoxelSize`) 4.0) 100.0))
  (`InstancedStaticMeshComponent.ClearInstances` (`self.HISM_GroupBillboard`))
  (for _array_element (`self.GroupDataArray`)
    (set `local.Mask0` 0.0)
    (set `local.Mask1` 0.0)
    (set `local.Mask2` 0.0)
    (set `local.Mask3` 0.0)
    (bind (_groupindex _groupx _groupy _groupz _voxelindices) (break `/Game/BluePrint/Data/ST_GroupData` _array_element))
    (for _array_element_2 _voxelindices
      (bind _returnvalue_3 (+ (mod (mod _array_element_2 _returnvalue) 4) (* (mod (mod (/ _array_element_2 _returnvalue) _returnvalue) 4) 4) (* (mod (/ _array_element_2 (* _returnvalue _returnvalue)) 4) 16)))
      (switch `int` (/ _returnvalue_3 16)
        (:`0`
          (bind _returnvalue_4 (`KismetMathLibrary.MultiplyMultiply_FloatFloat` 2.0 (`KismetMathLibrary.Conv_IntToDouble` (mod _returnvalue_3 16))))
          (set `local.Mask0` (+ (`local.Mask0`) _returnvalue_4)))
        (:`1`
          (set `local.Mask1` (+ (`local.Mask1`) _returnvalue_4)))
        (:`2`
          (set `local.Mask2` (+ (`local.Mask2`) _returnvalue_4)))
        (:`3`
          (set `local.Mask3` (+ (`local.Mask3`) _returnvalue_4)))))
    (if ShowBillboards
      (bind _returnvalue_5 (`KismetMathLibrary.MakeVector` (* (+ (`KismetMathLibrary.Conv_IntToDouble` (* _groupx 4)) 1.5) _voxelsize) (* (+ (`KismetMathLibrary.Conv_IntToDouble` (* _groupy 4)) 1.5) _voxelsize) (* (+ (`KismetMathLibrary.Conv_IntToDouble` (* _groupz 4)) 1.5) _voxelsize)))
      (bind _returnvalue_6 (`InstancedStaticMeshComponent.AddInstance` (`self.HISM_GroupBillboard`) (`KismetMathLibrary.MakeTransform` _returnvalue_5 (`KismetMathLibrary.ComposeRotators` (`KismetMathLibrary.FindLookAtRotation` _returnvalue_5 (`PlayerCameraManager.GetCameraLocation` (`GameplayStatics.GetPlayerCameraManager` 0))) (struct :`Pitch` 60.0 :`Roll` 30.0)) (`KismetMathLibrary.MakeVector` _returnvalue_2 _returnvalue_2 1.0)) false))
      ;[1 1 1] InstanceIndex
      (`InstancedStaticMeshComponent.SetCustomDataValue` (`self.HISM_GroupBillboard`) _returnvalue_6 0 (`local.Mask0`) false)
      (`InstancedStaticMeshComponent.SetCustomDataValue` (`self.HISM_GroupBillboard`) _returnvalue_6 1 (`local.Mask1`) false)
      (`InstancedStaticMeshComponent.SetCustomDataValue` (`self.HISM_GroupBillboard`) _returnvalue_6 2 (`local.Mask2`) false)
      (`InstancedStaticMeshComponent.SetCustomDataValue` (`self.HISM_GroupBillboard`) _returnvalue_6 3 (`local.Mask3`) true))))

(fn `IsVoxelOccupied`
  (params (Index :type Integer))
  (returns (Occupied :type Boolean))
  (return (`|GetArrayItem` (`self.VoxelMask`) Index)))

(fn `UserConstructionScript`)